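; BP_P_MainMenuPlayer is the player Blueprint for the TurboTetris main menu, handling input and level switching.
; Horizontal and Vertical axis inputs only print direction messages as placeholders, with positive horizontal values reported as left.
; Pressing L checks the current level name, opening the game level from the main menu or returning to the main menu from the credits.
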(event EventBeginPlay)

(event Collision|EventActorBeginOverlap
  (params (OtherActor :type Actor%20Object%20Reference)))

(event EventTick
  (params (DeltaSeconds :type Float%20%28single-precision%29)))

(event Input|AxisEvents|InputAxisHorizontal
  (params (AxisValue :type Float%20%28single-precision%29))
  (Math|Float|CompareFloat AxisValue 0.0
    (:>
      ;[1 1 1] Todo Implement logic here
      (Development|PrintString "LEFT PRESSED"))
    (:<
      (Development|PrintString "RIGHT PRESSED"))))

(event Input|AxisEvents|InputAxisVertical
  (params (AxisValue :type Float%20%28single-precision%29))
  (Math|Float|CompareFloat AxisValue 0.0
    (:>
      ;[1 1 1] Todo Implement logic here
      (Development|PrintString "UP PRESSED"))
    (:<
      (Development|PrintString "DOWN PRESSED"))))

(event Input|KeyboardEvents|L
  (params (Key :type Key%20Structure :default "None"))
  (:Pressed
    (bind _returnvalue (Game|GetCurrentLevelName true))
    (switch string _returnvalue
      (:L_MainMenu
        (Game|OpenLevel(byObjectReference) "/Game/TurboTetris/Levels/L_Game.L_Game"))
      (:L_Credits
        (Game|OpenLevel(byObjectReference) "/Game/TurboTetris/Levels/L_MainMenu.L_MainMenu")))))

(fn ConstructionScript)