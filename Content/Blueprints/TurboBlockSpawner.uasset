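; Spawner actor for a Tetris-style game that creates TurboTetrisBlock actors one at a time at its SpawnLocation.
; After a short startup delay it spawns a block, stores it as current and binds to its block-stopped event.
; SpawnNextBlock repeats that spawn unless a debug-drawn box trace at the spawn point finds world static or dynamic objects, in which case it prints that the grid is full.
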(event Custom|StartGame
  (Utilities|FlowControl|Delay 0.1)
  (bind _returnvalue (Game|SpawnActorfromClass "/Game/Blueprints/TurboTetrisBlock.TurboTetrisBlock_C" (Transformation|GetWorldTransform (Variables|Default|GetSpawnLocation)) "Undefined" 0 1.0 0 0))
  (bind _output_get (Variables|Default|SetCurrentTetrisBlock _returnvalue))
  (EventDispatchers|BindEventtoBlockStopped _output_get (EventDispatchers|CreateEvent :!event Custom|SpawnNextBlock)))

(event Custom|SpawnNextBlock
  (bind _gridisfull (CallFunction|CheckifGridIsFull))
  (if _gridisfull
    (Development|PrintString "FGrid Is Full")
    (else
      (bind _returnvalue (Game|SpawnActorfromClass "/Game/Blueprints/TurboTetrisBlock.TurboTetrisBlock_C" (Transformation|GetWorldTransform (Variables|Default|GetSpawnLocation)) "Undefined" 0 1.0 0 0))
      (bind _output_get (Variables|Default|SetCurrentTetrisBlock _returnvalue))
      (EventDispatchers|BindEventtoBlockStopped _output_get (EventDispatchers|CreateEvent :!event Custom|SpawnNextBlock)))))

(event EventBeginPlay
  (Utilities|FlowControl|Delay 1.0)
  (CallFunction|StartGame))

(event Collision|EventActorBeginOverlap
  (params (OtherActor :type Actor%20Object%20Reference)))

(event EventTick
  (params (DeltaSeconds :type Float%20%28single-precision%29)))

(fn ConstructionScript)

(fn CheckifGridIsFull
  (bind _spawnlocation (Variables|Default|GetSpawnLocation))
  (bind _returnvalue (Transformation|GetWorldLocation _spawnlocation))
  (bind _returnvalue_2 (Class|KismetSystemLibrary|BoxTraceMultiforObjects _returnvalue _returnvalue "50.000000,1000.000000,50.000000" "0, 0, 0" (Utilities|Array|MakeArray "ObjectTypeQuery1" "ObjectTypeQuery2") false 0 "ForDuration" true))
  (return _returnvalue_2))