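; SplineObjectBP is an actor that moves a Scene component along its own spline in a continuous loop.
; The construction script caches the spline length and sets the component's world location and rotation at the starting distance.
; Tick advances the distance by Speed times delta time, resets it to zero on reaching the end, and updates only location, so rotation does not follow the path at runtime.
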(event EventBeginPlay)

(event Collision|EventActorBeginOverlap
  (params (OtherActor :type Actor%20Object%20Reference)))

(event EventTick
  (params (DeltaSeconds :type Float%20%28single-precision%29))
  (Variables|Default|SetDistanceAlongSpline (+ (Variables|Default|GetDistanceAlongSpline) (* (Variables|Default|GetSpeed) DeltaSeconds)))
  (Math|Float|CompareFloat (Variables|Default|GetDistanceAlongSpline) (Variables|Default|GetSplineLength)
    (:>
      (Variables|Default|SetDistanceAlongSpline 0.0 :!label _label))
    (:==
      (goto _label))
    (:<
      _))
  (Transformation|SetWorldLocation (Variables|Default|GetScene) (Spline|GetLocationatDistanceAlongSpline (Variables|Default|GetSpline) (Variables|Default|GetDistanceAlongSpline) "World") false false))

(fn ConstructionScript
  (bind _spline (Variables|Default|GetSpline))
  (bind _distancealongspline (Variables|Default|GetDistanceAlongSpline))
  (Variables|Default|SetSplineLength (Spline|GetSplineLength (Variables|Default|GetSpline)))
  (Transformation|SetWorldLocation (Variables|Default|GetScene) (Spline|GetLocationatDistanceAlongSpline _spline _distancealongspline "World") false false)
  (Transformation|SetWorldRotation (Variables|Default|GetScene) (Spline|GetRotationatDistanceAlongSpline _spline _distancealongspline "World") false false))