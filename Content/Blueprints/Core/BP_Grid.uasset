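; BP_Grid is a grid actor that builds and manages squares, each with an occupied state and soil type.
; On BeginPlay, nested loops spawn BP_Row actors into SquaresGrid and fill each row's Squares array with spawned BP_Square actors.
; Spawn locations are constants, not derived from the loop indices.
; GetSquare looks up a square by row and column, and SetSquare uses it to write that square's occupancy and soil.
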(event EventBeginPlay
  (for _index (range 0 (Variables|Default|GetNumberOfRows))
    (bind _returnvalue (Game|SpawnActorfromClass "/Game/Blueprints/Core/BP_Row.BP_Row_C" (Math|Transform|MakeTransform "0,1000.000000, 0" "0, 0, 0" "1,1,1") "Undefined" 0 0))
    (Utilities|Array|AddUnique (Variables|Default|GetSquaresGrid) _returnvalue)
    (for _index_2 (range 0 (Variables|Default|GetNumberOfColumns))
      (bind _returnvalue_2 (Game|SpawnActorfromClass "/Game/Blueprints/Core/BP_Square.BP_Square_C" (Math|Transform|MakeTransform "1000.000000, 0, 0" "0, 0, 0" "1,1,1") "Undefined" 0 0))
      (Utilities|Array|Add (Variables|/Game/Blueprints/Core/BP_Row.BP_Row_C|GetSquares _returnvalue) _returnvalue_2))))

(fn ConstructionScript)

(fn GetSquare
  (params (Row :type Integer) (Column :type Integer))
  (return (Utilities|Array|Get(acopy) (Variables|/Game/Blueprints/Core/BP_Row.BP_Row_C|GetSquares (Utilities|Array|Get(acopy) (Variables|Default|GetSquaresGrid) Row)) Column)))

(fn SetSquare
  (params (Row :type Integer) (Column :type Integer) (Occupied :type Boolean) (Soil :type SoilTypes%20Enum :default "NewEnumerator0"))
  (bind _squareref (CallFunction|GetSquare Row Column))
  (Variables|/Game/Blueprints/Core/BP_Square.BP_Square_C|SetOccupied _squareref Occupied)
  (Variables|/Game/Blueprints/Core/BP_Square.BP_Square_C|SetSoilType _squareref Soil))