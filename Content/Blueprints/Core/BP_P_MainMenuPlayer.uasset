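; Player Blueprint for the main menu and credits screens that moves between levels on a Space or L key press.
; Both keys share a switch on the current level name.
; In the main menu it turns on physics for every TURBOISLAND element, then opens the game level after a short delay, while in credits it opens the main menu.
; The four Turbo input actions only print debug strings.
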(event EventBeginPlay)

(event Collision|EventActorBeginOverlap
  (params (OtherActor :type Actor%20Object%20Reference)))

(event EventTick
  (params (DeltaSeconds :type Float%20%28single-precision%29)))

(event Input|ActionEvents|InputActionTurboLeft
  (params (Key :type Key%20Structure :default "None"))
  (:Pressed
    ;[1 1 1] Todo Implement logic here
    (Development|PrintString "LEFT PRESSED")))

(event Input|ActionEvents|InputActionTurboRight
  (params (Key :type Key%20Structure :default "None"))
  (:Pressed
    ;[1 1 1] Todo Implement logic here
    (Development|PrintString "RIGHT PRESSED")))

(event Input|ActionEvents|InputActionTurboDown
  (params (Key :type Key%20Structure :default "None"))
  (:Pressed
    ;[1 1 1] Todo Implement logic here
    (Development|PrintString "DOWN PRESSED")))

(event Input|ActionEvents|InputActionTurboRotate
  (params (Key :type Key%20Structure :default "None"))
  (:Pressed
    ;[1 1 1] Todo Implement logic here
    (Development|PrintString "UP PRESSED")))

(event Input|KeyboardEvents|L
  (params (Key :type Key%20Structure :default "None"))
  (:Pressed
    (bind _returnvalue (Game|GetCurrentLevelName true))
    (switch string _returnvalue
      (:L_MainMenu
        (for _array_element (Variables|Default|GetTURBOISLAND)
          (Default|TogglePhysics _array_element true))
        (Utilities|FlowControl|Delay 1.5)
        (Game|OpenLevel(byObjectReference) "/Game/Maps/Build/Game/L_P_Game.L_P_Game"))
      (:L_Credits
        (Game|OpenLevel(byObjectReference) "/Game/Maps/Build/L_MainMenu.L_MainMenu")))))

(event Input|KeyboardEvents|SpaceBar
  (params (Key :type Key%20Structure :default "None"))
  (:Pressed
    (bind _returnvalue (Game|GetCurrentLevelName true))
    (switch string _returnvalue
      (:L_MainMenu
        (for _array_element (Variables|Default|GetTURBOISLAND)
          (Default|TogglePhysics _array_element true))
        (Utilities|FlowControl|Delay 1.5)
        (Game|OpenLevel(byObjectReference) "/Game/Maps/Build/Game/L_P_Game.L_P_Game"))
      (:L_Credits
        (Game|OpenLevel(byObjectReference) "/Game/Maps/Build/L_MainMenu.L_MainMenu")))))

(fn ConstructionScript)