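; A Tetris piece of four cubes with a random or preset shape and a soil type that sets its material and landing behavior.
; It steps down until box traces block it, which also validate rotations.
; Sand then crumbles cube by cube, Clay stays rigid and Silt shakes until a later spawn collapses it, prompting Clay pieces to fall again.
; Stopped pieces report grid positions through the BlockStopped call.
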(event Custom|DropSiltBlock
  (Utilities|FlowControl|MultiGate false false -1
    (:Out%201
      (Audio|Components|Audio|Stop (Variables|Default|GetShakingTimeline))
      (bind _didanyblocksmove_ (CallFunction|MoveBlocksDown :!label _label))
      (if _didanyblocksmove_
        (Utilities|FlowControl|RetriggerableDelay 0.1)
        (goto _label)
        (else
          (bind _outactors (Actor|GetAllActorsOfClass "TurboTetrisBlock_C"))
          (for _array_element _outactors
            (CallFunction|CheckifBlocksShouldDrop _array_element)))))))

(event Custom|StartShakingTimeline
  (bind (_primitives _startlocations _endlocations) (CallFunction|GetTimelineVariables))
  (bind _newtrack_0 (Timeline|ShakingTimeline PlayFromStart)
    (:Update
      (for (_array_element _array_index) _primitives
        (Transformation|SetWorldLocation _array_element (Math|Vector|Lerp(Vector) (Utilities|Array|Get(acopy) _startlocations _array_index) (Utilities|Array|Get(acopy) _endlocations _array_index) _newtrack_0) false false)))))

(event Custom|CheckIfBlocksShouldDrop
  (switch Utilities|FlowControl|Switch|SwitchonSoilTypes (Variables|Default|GetSoilType)
    (:NewEnumerator2
      (Utilities|FlowControl|RetriggerableDelay 0.1 :!label _label)
      (bind _movesuccessfull (CallFunction|MoveObjectinDirection "0, 0,-100.000000" "None"))
      (if _movesuccessfull
        (goto _label)))))

(event EventBeginPlay
  (if (not (Variables|Debug|GetbUsedFixedVariable))
    (Utilities|FlowControl|RetriggerableDelay (Variables|Default|GetMovementDelay) :!label _label)
    (bind _movesuccessfull (CallFunction|MoveObjectinDirection "0, 0,-100.000000" "None"))
    (if _movesuccessfull
      (goto _label)
      (else
        (switch Utilities|FlowControl|Switch|SwitchonSoilTypes (Variables|Default|GetSoilType)
          (:NewEnumerator0
            (bind _didanyblocksmove_ (CallFunction|MoveBlocksDown :!label _label_2))
            (if _didanyblocksmove_
              (Utilities|FlowControl|RetriggerableDelay 0.1)
              (goto _label_2)
              (else
                _)))
          (:NewEnumerator1
            (EventDispatchers|BindEventtoNewBlockSpawned (Variables|Default|GetBlockSpawner) (delegate Custom|DropSiltBlock))
            (CallFunction|StartShakingTimeline))
          (:NewEnumerator2
            _))
        (Default|CallBlockStopped self (CallFunction|GetGridPositions))
        (Development|PrintString "BlockStopped")))))

(fn ConstructionScript
  (Utilities|FlowControl|Sequence
    (:then_0
      (if (Variables|Debug|GetbUsedFixedVariable)
        _
        (else
          (Variables|Default|SetType (Math|Random|RandomIntegerinRange 0 6))))
      (for (_array_element _array_index) (Utilities|Select :Index (Variables|Default|GetType) :Option%200 (LocalVariables|GetTypeO) :Option%201 (LocalVariables|GetTypeI) :Option%202 (LocalVariables|GetTypeS) :Option%203 (LocalVariables|GetTypeZ) :Option%204 (LocalVariables|GetTypeL) :Option%205 (LocalVariables|GetTypeJ) :Option%206 (LocalVariables|GetTypeT))
        (Transformation|SetRelativeLocation (Utilities|Array|Get(acopy) (Utilities|Array|MakeArray (Variables|Default|GetBlock1) (Variables|Default|GetBlock2) (Variables|Default|GetBlock3) (Variables|Default|GetBlock4)) _array_index) _array_element false false)))
    (:then_1
      (for _array_element_2 (Utilities|Array|MakeArray (Variables|Default|GetBlock1) (Variables|Default|GetBlock2) (Variables|Default|GetBlock3) (Variables|Default|GetBlock4))
        (Rendering|Material|SetMaterial _array_element_2 0 (Utilities|Select :Index (Variables|Default|GetSoilType) :NewEnumerator3 0 :NewEnumerator0 "/Game/StarterContent/Materials/M_Rock_Sandstone.M_Rock_Sandstone" :NewEnumerator1 "/Game/StarterContent/Materials/M_Metal_Rust.M_Metal_Rust" :NewEnumerator2 "/Game/StarterContent/Materials/M_Tech_Hex_Tile.M_Tech_Hex_Tile" :NewEnumerator4 0)))
      (Components|Timeline|SetPlayRate (Variables|Default|GetShakingTimeline) 5.0))))

(fn MoveObjectinDirection
  (params (Offset :type Vector) (DebugType :type EDrawDebugTrace%20Enum :default "None"))
  (for _array_element (Utilities|Array|MakeArray (Variables|Default|GetBlock1) (Variables|Default|GetBlock2) (Variables|Default|GetBlock3) (Variables|Default|GetBlock4))
    (bind _returnvalue (Class|KismetSystemLibrary|BoxTraceMultiforObjects (+ (Transformation|GetWorldLocation _array_element) Offset) (+ (Transformation|GetWorldLocation _array_element) Offset) (Math|Conversions|ToVector(Float) (Math|Float|MakeLiteralFloat 45.0)) "0, 0, 0" (Utilities|Array|MakeArray "ObjectTypeQuery1" "ObjectTypeQuery2") false 0 DebugType true))
    (if _returnvalue
      (LocalVariables|SetBlocked true)))
  (if (LocalVariables|GetBlocked)
    (return false)
    (else
      (Transformation|AddActorWorldOffset Offset)
      (return true))))

(fn Rotate
  (params (Clockwise :type Boolean))
  (if (!= (Variables|Default|GetType) 0)
    (Class|Actor|AddActorWorldRotation (select Clockwise "0, 0,-90.000000" "0.000000,0.000000,90.000000"))
    (for _array_element (Utilities|Array|MakeArray (Variables|Default|GetBlock1) (Variables|Default|GetBlock2) (Variables|Default|GetBlock3) (Variables|Default|GetBlock4))
      (bind _returnvalue (Class|KismetSystemLibrary|BoxTraceMultiforObjects (Transformation|GetWorldLocation _array_element) (Transformation|GetWorldLocation _array_element) (Math|Conversions|ToVector(Float) (Math|Float|MakeLiteralFloat 45.0)) "0, 0, 0" (Utilities|Array|MakeArray "ObjectTypeQuery1" "ObjectTypeQuery2") false 0 "None" true))
      (if _returnvalue
        (LocalVariables|SetBlocked true)))
    (Utilities|FlowControl|Sequence
      (:then_0
        (if (LocalVariables|GetBlocked)
          (Class|Actor|AddActorWorldRotation (select (not Clockwise) "0, 0,-90.000000" "0.000000,0.000000,90.000000"))))
      (:then_1
        (return (LocalVariables|GetBlocked))))))

(fn GetGridPositions
  (for _array_element (Utilities|Array|MakeArray (Variables|Default|GetBlock1) (Variables|Default|GetBlock2) (Variables|Default|GetBlock3) (Variables|Default|GetBlock4))
    (Utilities|Array|Add (LocalVariables|GetTempGridPositions) (Utilities|Struct|MakeGridPosition (Math|Vector2D|MakeVector2D (Math|Conversions|ToFloat(Integer) (Math|Integer|Absolute(Integer) (Math|Float|Truncate (.y (/ (- (Transformation|GetWorldLocation _array_element) (Transformation|GetWorldLocation (Variables|/Game/Blueprints/TurboBlockSpawner.TurboBlockSpawner_C|Get1X1Location (Variables|Default|GetBlockSpawner)))) 1e+02))))) (Math|Conversions|ToFloat(Integer) (Math|Integer|Absolute(Integer) (Math|Float|Truncate (.z (/ (- (Transformation|GetWorldLocation _array_element) (Transformation|GetWorldLocation (Variables|/Game/Blueprints/TurboBlockSpawner.TurboBlockSpawner_C|Get1X1Location (Variables|Default|GetBlockSpawner)))) 1e+02)))))) (Variables|Default|GetSoilType)))
    (if (Variables|Debug|GetbDebug)
      (Development|PrintString (Utilities|String|Append "X = " (Utilities|String|ToString(Integer) (Math|Integer|Absolute(Integer) (Math|Float|Truncate (.y (/ (- (Transformation|GetWorldLocation _array_element) (Transformation|GetWorldLocation (Variables|/Game/Blueprints/TurboBlockSpawner.TurboBlockSpawner_C|Get1X1Location (Variables|Default|GetBlockSpawner)))) 1e+02))))) " Y = " (Utilities|String|ToString(Integer) (Math|Integer|Absolute(Integer) (Math|Float|Truncate (.z (/ (- (Transformation|GetWorldLocation _array_element) (Transformation|GetWorldLocation (Variables|/Game/Blueprints/TurboBlockSpawner.TurboBlockSpawner_C|Get1X1Location (Variables|Default|GetBlockSpawner)))) 1e+02)))))))))
  (return (LocalVariables|GetTempGridPositions)))

(fn MoveBlocksDown
  (for _array_element (Utilities|Array|MakeArray (Variables|Default|GetBlock2) (Variables|Default|GetBlock3) (Variables|Default|GetBlock4) (Variables|Default|GetBlock1))
    (LocalVariables|SetBlockFromArray _array_element)
    (bind _returnvalue (Class|KismetSystemLibrary|BoxTraceMultiforObjects (+ (Transformation|GetWorldLocation (LocalVariables|GetBlockFromArray)) "0, 0,-100.000000") (+ (Transformation|GetWorldLocation (LocalVariables|GetBlockFromArray)) "0, 0,-100.000000") (Math|Conversions|ToVector(Float) (Math|Float|MakeLiteralFloat 25.0)) "0, 0, 0" (Utilities|Array|MakeArray "ObjectTypeQuery2" "ObjectTypeQuery1") false 0 "None" false))
    (if (not _returnvalue)
      (Transformation|AddWorldOffset (LocalVariables|GetBlockFromArray) "0, 0,-100.000000" false false)
      (LocalVariables|SetBlocksMoved true)))
  (return (LocalVariables|GetBlocksMoved)))

(fn GetTimelineVariables
  (for _array_element (Utilities|Array|MakeArray (Variables|Default|GetBlock2) (Variables|Default|GetBlock3) (Variables|Default|GetBlock4) (Variables|Default|GetBlock1))
    (Utilities|Array|Add (LocalVariables|GetTemp_StartLocations) (Transformation|GetWorldLocation _array_element))
    (Utilities|Array|Add (LocalVariables|GetTemp_EndLocations) (+ (Transformation|GetWorldLocation _array_element) (* (Math|Random|RandomUnitVector) (Math|Random|RandomFloatinRange 5.0 1e+01)))))
  (return (Utilities|Array|MakeArray (Variables|Default|GetBlock2) (Variables|Default|GetBlock3) (Variables|Default|GetBlock4) (Variables|Default|GetBlock1)) (LocalVariables|GetTemp_StartLocations) (LocalVariables|GetTemp_EndLocations)))