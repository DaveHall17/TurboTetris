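; SoundBox is an actor that animates a cone's scale and a static mesh's position when play begins.
; BeginPlay stores the mesh's start location, then fires a custom event that plays a timeline to set the cone's relative scale.
; A second timeline teleports the mesh along the world XY diagonal, offset from that start by the scaled track value.
; Tick is unused, and the graph contains no audio logic despite the name.
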(event Custom|coneevent
  (bind _newtrack_0 (Timeline|Timeline_0 PlayFromStart)
    (:Update
      (Transformation|SetRelativeScale3D (Variables|Default|GetCone) (Math|Conversions|ToVector(Float) _newtrack_0)))))

(event EventBeginPlay
  (Variables|Default|Setstartpos (Transformation|GetWorldLocation (Variables|Debug|GetStaticMeshComponent)))
  (CallFunction|Coneevent)
  (bind _newtrack_0 (Timeline|Timeline_1 Play)
    (:Update
      (Transformation|SetWorldLocation (Variables|Debug|GetStaticMeshComponent) (Math|Vector|MakeVector (+ (.x (Variables|Default|Getstartpos)) (* _newtrack_0 1e+01)) (+ (.y (Variables|Default|Getstartpos)) (* _newtrack_0 1e+01)) (.z (Variables|Default|Getstartpos))) false true))))

(event EventTick
  (params (DeltaSeconds :type Float%20%28single-precision%29)))

(fn ConstructionScript)