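; TurboPawn is the player pawn for a Tetris-style game, moving the falling block down, left or right.
; On BeginPlay it finds the TurboBlockSpawner and enables input, then each action calls MoveObjectInDirection on the spawner's CurrentTetrisBlock.
; Each action runs through its own InputMacro, a Gate and RetriggerableDelay loop that auto-repeats while held, with shrinking intervals down to a minimum, and resets on release.
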(event EventBeginPlay
  (bind _returnvalue (Game|GetPlayerController 0))
  (bind _outactors (Actor|GetAllActorsOfClass "/Game/Blueprints/TurboBlockSpawner.TurboBlockSpawner_C"))
  (Variables|Default|SetBlockSpawner (Utilities|Array|Get(acopy) _outactors))
  (Input|EnableInput _returnvalue)
  (Input|SetInputModeGameOnly _returnvalue))

(event Input|ActionEvents|InputActionTurboDown
  (params (Key :type Key%20Structure :default "None"))
  (bind _blockspawner (Variables|Default|GetBlockSpawner))
  (:Pressed
    (Utilities|InputMacro :!label _label
      (:Out
        (Development|PrintString "Down")
        (Utilities|IsValid _blockspawner
          (:Is%20Valid
            (Default|MoveObjectinDirection (Variables|/Game/Blueprints/TurboBlockSpawner.TurboBlockSpawner_C|GetCurrentTetrisBlock _blockspawner) "0.000000,0.000000,-100.000000" "ForDuration"))
          (:Is%20Not%20Valid
            (Development|PrintString "Not valid"))))))
  (:Released
    (goto _label Released)))

(event Input|ActionEvents|InputActionTurboLeft
  (params (Key :type Key%20Structure :default "None"))
  (bind _blockspawner (Variables|Default|GetBlockSpawner))
  (:Pressed
    (Utilities|InputMacro :!label _label
      (:Out
        (Development|PrintString "Left")
        (Utilities|IsValid _blockspawner
          (:Is%20Valid
            (Default|MoveObjectinDirection (Variables|/Game/Blueprints/TurboBlockSpawner.TurboBlockSpawner_C|GetCurrentTetrisBlock _blockspawner) "0.000000,-100.000000, 0" "ForDuration"))
          (:Is%20Not%20Valid
            (Development|PrintString "Not valid"))))))
  (:Released
    (goto _label Released)))

(event Input|ActionEvents|InputActionTurboRight
  (params (Key :type Key%20Structure :default "None"))
  (bind _blockspawner (Variables|Default|GetBlockSpawner))
  (:Pressed
    (Utilities|InputMacro :!label _label
      (:Out
        (Development|PrintString "Right")
        (Utilities|IsValid _blockspawner
          (:Is%20Valid
            (Default|MoveObjectinDirection (Variables|/Game/Blueprints/TurboBlockSpawner.TurboBlockSpawner_C|GetCurrentTetrisBlock _blockspawner) "0.000000,100.000000, 0" "ForDuration"))
          (:Is%20Not%20Valid
            (Development|PrintString "Not valid"))))))
  (:Released
    (goto _label Released)))

(event Input|ActionEvents|InputActionTurboRotate
  (params (Key :type Key%20Structure :default "None")))

(fn ConstructionScript)