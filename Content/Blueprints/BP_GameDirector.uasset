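; BP_GameDirector is a director actor that watches the TurboBlockSpawner for a full grid.
; On BeginPlay it finds the spawner in the level if the reference is unset, then binds to its GridIsFull event.
; When that fires, it forwards to ExecuteGridIsFull, which currently only prints a debug message.
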(event Custom|Grid%20IsFull
  (CallFunction|ExecuteGridIsFull))

(event Custom|Execute%20GridIsFull
  (Development|PrintString "GRID IS FULL"))

(event EventBeginPlay
  (CallFunction|GetReferences)
  (bind _turboblockspawner (Variables|References|GetTurboBlockSpawner)
    (:then
      (EventDispatchers|BindEventtoGridIsFull _turboblockspawner (delegate Custom|Grid%20IsFull)))
    (:else)))

(event Collision|EventActorBeginOverlap
  (params (OtherActor :type Actor%20Object%20Reference)))

(event EventTick
  (params (DeltaSeconds :type Float%20%28single-precision%29)))

(fn ConstructionScript)

(fn GetReferences
  (Utilities|FlowControl|Sequence
    (:then_0
      (Variables|References|GetTurboBlockSpawner
        (:then)
        (:else
          (bind _returnvalue (Actor|GetActorOfClass "/Game/Blueprints/TurboBlockSpawner.TurboBlockSpawner_C"))
          (Variables|References|SetTurboBlockSpawner _returnvalue))))))