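; Explosion actor for a burning bin that blasts nearby DancingCharacter actors when its Explode event is called.
; Each character overlapping the Sphere is ragdolled and launched by a velocity-change impulse, aimed from the actor toward a point high above it for strong lift, with the vector debug-printed.
; The bin mesh becomes physical and tumbles away with fixed impulses, alongside a 2D sound, a scaled-up explosion particle and deactivation of the fire effect.
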(event Custom|Explode
  (bind _binmesh (Variables|Default|GetBinMesh))
  (Audio|PlaySound2D "/Game/StarterContent/Audio/Explosion02.Explosion02" 1.0 1.0 0.0 0 0)
  (for _array_element (Collision|GetOverlappingActors (Variables|Default|GetSphere) 0 :!class /Script/Engine.PrimitiveComponent)
    (bind _asdancing_character (Utilities|Casting|CastToDancingCharacter _array_element))
    (Default|Ragdoll _asdancing_character)
    (Physics|AddImpulse (Variables|/Game/Blueprints/DancingCharacter.DancingCharacter_C|GetSkeletalMesh _asdancing_character) (* (Math|Rotator|GetRotationXVector (Math|Rotator|FindLookatRotation (Transformation|GetWorldLocation (Variables|Default|GetDefaultSceneRoot)) (+ (Transformation|GetWorldLocation (Variables|/Game/Blueprints/DancingCharacter.DancingCharacter_C|GetSkeletalMesh _asdancing_character)) "0, 0,1000.000000"))) 2e+04) "None" true)
    (Development|PrintString (Utilities|String|ToString(Vector) (* (Math|Rotator|GetRotationXVector (Math|Rotator|FindLookatRotation (Transformation|GetWorldLocation (Variables|Default|GetDefaultSceneRoot)) (+ (Transformation|GetWorldLocation (Variables|/Game/Blueprints/DancingCharacter.DancingCharacter_C|GetSkeletalMesh _asdancing_character)) "0, 0,1000.000000"))) 2e+04))))
  (Physics|SetSimulatePhysics _binmesh true)
  (Class|PrimitiveComponent|AddAngularImpulseinRadians _binmesh "100.000000,100.000000, 0" "None" true)
  (Physics|AddImpulse _binmesh "200.000000,500.000000,100.000000" "None" true)
  (Effects|SpawnEmitteratLocation "/Game/StarterContent/Particles/P_Explosion.P_Explosion" (Transformation|GetWorldLocation (Variables|Default|GetScene)) "0, 0, 0" (Math|Conversions|ToVector(Float) (Math|Float|MakeLiteralFloat 2e+01)))
  (Components|Activation|Deactivate (Variables|Default|GetFireSystem)))

(fn ConstructionScript)