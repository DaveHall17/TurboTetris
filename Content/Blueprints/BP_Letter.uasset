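; BP_Letter is a 3D text actor whose physics the main menu can toggle.
; The construction script applies its text plus front and extrude materials to Text3D, leaving bevel and back material inputs unset.
; On BeginPlay it disables simulation on its Box, then registers itself in the BP_P_MainMenuPlayer pawn's PhysicsLetters array.
; TogglePhysics switches Box simulation on or off.
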(event Custom|Toggle%20Physics
  (params (bSimulate :type Boolean))
  (Physics|SetSimulatePhysics (Variables|Default|GetBox) bSimulate))

(event EventBeginPlay
  (CallFunction|TogglePhysics false)
  (bind _asbp_p_main_menu_player (Utilities|Casting|CastToBP_P_MainMenuPlayer (Game|Player|GetPlayerPawn 0)))
  (Utilities|Array|AddUnique (Variables|/Game/Blueprints/Core/BP_P_MainMenuPlayer.BP_P_MainMenuPlayer_C|GetPhysicsLetters _asbp_p_main_menu_player) self))

(event Collision|EventActorBeginOverlap
  (params (OtherActor :type Actor%20Object%20Reference)))

(event EventTick
  (params (DeltaSeconds :type Float%20%28single-precision%29)))

(fn ConstructionScript
  (Class|Text3DComponent|SetText (Variables|Default|GetText3D) (Variables|Default|GetText))
  (Utilities|FlowControl|Sequence
    (:then_0
      (Class|Text3DComponent|SetFrontMaterial (Variables|Default|GetText3D) (Variables|Materials|GetFontMaterial)))
    (:then_1
      (Class|Text3DComponent|SetExtrudeMaterial (Variables|Default|GetText3D) (Variables|Materials|GetExtrudeMaterials)))
    (:then_2
      (Class|Text3DComponent|SetBevelMaterial (Variables|Default|GetText3D)))
    (:then_3
      (Class|Text3DComponent|SetBackMaterial (Variables|Default|GetText3D)))))