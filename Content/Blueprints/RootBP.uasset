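; Tree actor that, once per game on CheckRoots, grows roots through connected Sand and Silt Tetris blocks and scores the result.
; GetRoots flood-fills outward from its origin using box traces on neighboring cells, capped by a DoN, adding a root mesh component per valid cell.
; CheckRoots then reveals the roots one by one on a retriggerable-delay loop, enlarging the tree and updating the billboard score each step.
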(event Custom|CheckRoots
  (bind _rootmeshes (Variables|Default|GetRootMeshes))
  (bind _index (Variables|Default|GetIndex))
  (bind _index_2 (Variables|Default|GetIndex))
  (bind _output (Utilities|Array|Get(acopy) _rootmeshes _index))
  (Utilities|FlowControl|DoOnce false
    (:Completed
      (Audio|SpawnSound2D "/Game/SFX/tree.tree" 1.0 1.0 0.0 0)
      (CallFunction|GetRoots)
      (Utilities|IsValid _output :!label _label
        (:Is%20Valid
          (Development|SetHiddeninGame _output false false)
          (Math|Integer|IncrementInt _index_2
            (:%20%20
              (Utilities|FlowControl|RetriggerableDelay 0.1)
              (Transformation|SetRelativeScale3D (Variables|Default|GetTreeMesh) (Math|Conversions|ToVector(Float) (* _index_2 0.25)))
              (Default|UpdateScore (Variables|Default|GetBillBoard) (Variables|Default|GetIndex))
              (goto _label))))))))

(event Collision|EventActorBeginOverlap
  (params (OtherActor :type Actor%20Object%20Reference)))

(event EventTick
  (params (DeltaSeconds :type Float%20%28single-precision%29)))

(event EventBeginPlay)

(fn ConstructionScript)

(fn GetRoots
  (bind _newlocationstocheck (LocalVariables|GetNewLocationsToCheck))
  (bind _returnvalue (Utilities|Array|Length _newlocationstocheck))
  (Utilities|FlowControl|Sequence
    (:then_0
      (Variables|Default|SetLocationsToCheck (Utilities|Array|MakeArray "0, 0, 0"))
      (for _array_element (Variables|Default|GetLocationsToCheck) :!label _label
        (for _array_element_2 (Variables|Default|GetDirectionsToCheck)
          (bind _output_get (LocalVariables|SetRelativeLocationToCheck (+ _array_element_2 _array_element)))
          (if (not (Utilities|Array|ContainsItem (LocalVariables|GetSpacesUsed) _output_get))
            (Utilities|FlowControl|DoN 500
              (:Exit
                (bind _outhit (Class|KismetSystemLibrary|BoxTraceSingleforObjects (Math|Transform|TransformLocation (Transformation|GetActorTransform) (LocalVariables|GetRelativeLocationToCheck)) (Math|Transform|TransformLocation (Transformation|GetActorTransform) (LocalVariables|GetRelativeLocationToCheck)) "55.000000,40.000000,40.000000" "0, 0, 0" (Utilities|Array|MakeArray "ObjectTypeQuery2") false 0 "None" true))
                (bind _asturbo_tetris_block (Utilities|Casting|CastToTurboTetrisBlock (.HitActor (Collision|BreakHitResult _outhit))))
                (switch Utilities|FlowControl|Switch|SwitchonSoilTypes (Variables|/Game/Blueprints/TurboTetrisBlock.TurboTetrisBlock_C|GetSoilType _asturbo_tetris_block)
                  (:NewEnumerator0
                    _)
                  (:NewEnumerator1
                    _))
                (bind _returnvalue_2 (AddComponent|AddInstancedStaticMeshComponent false (Math|Transform|MakeTransform (+ (LocalVariables|GetRelativeLocationToCheck) "-50.000000,10.000000,-50.000000"))))
                (Utilities|Array|Add (Variables|Default|GetRootMeshes) _returnvalue_2)
                (Utilities|Array|Add (LocalVariables|GetNewLocationsToCheck) (LocalVariables|GetRelativeLocationToCheck))
                (Utilities|Array|Add (LocalVariables|GetSpacesUsed) (LocalVariables|GetRelativeLocationToCheck)))))))
      (Development|PrintString (Utilities|String|Append (Utilities|String|ToString(Integer) _returnvalue) " locations to check"))
      (Math|Integer|CompareInt _returnvalue
        (:>
          (Utilities|Array|Clear (Variables|Default|GetLocationsToCheck))
          (Variables|Default|SetLocationsToCheck (LocalVariables|GetNewLocationsToCheck))
          (Utilities|Array|Clear (LocalVariables|GetNewLocationsToCheck))
          (Development|PrintString (Utilities|String|Append "Locations = " (Utilities|String|ToString(Integer) (Utilities|Array|Length (Variables|Default|GetLocationsToCheck))) " New locations = " (Utilities|String|ToString(Integer) (Utilities|Array|Length (LocalVariables|GetNewLocationsToCheck)))))
          (goto _label))))
    (:then_1
      (Development|PrintString (Utilities|String|Append (Utilities|String|ToString(Integer) (Utilities|Array|Length (Variables|Default|GetRootMeshes))) "Rootas")))))